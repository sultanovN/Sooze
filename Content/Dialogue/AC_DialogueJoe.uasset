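; Dialogue component for NPC Joe (Джо), who asks the player to deliver a letter to Leila across the flooded island.
; Overrides Dialogue, switching on the active branch through intro, quest given, Sergey hint and delivered stages.
; Chained AddDialogue nodes drive options and montages; the opening line's Updated state walks Joe toward the player.
; Completion checks LetterDeliv on BP_NPCTest's dialogue component; later idle lines are randomized.
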(fn Dialogue
  (|CallParentFunction)
  (switch name (Variables|Default|GetActiveDialogueBranch)
    (:Default
      (bind _state (CallFunction|AddDialogue "Джо" "Простите!"))
      (switch Utilities|FlowControl|Switch|SwitchonEnum_DialogueState _state
        (:NewEnumerator0
          (bind _state_2 (CallFunction|AddDialogue "Джо" "Мне нужна ваша помощь!"))
          (switch Utilities|FlowControl|Switch|SwitchonEnum_DialogueState _state_2
            (:NewEnumerator0
              (bind _state_3 (CallFunction|AddDialogue "Джо" "Мне срочно надо доставить письмо на другую сторону острова"))
              (switch Utilities|FlowControl|Switch|SwitchonEnum_DialogueState _state_3
                (:NewEnumerator0
                  (bind _state_4 (CallFunction|AddDialogue "Джо" "Но вот беда, дорогу туда потопило от растоявшего снега с вершины горы"))
                  (switch Utilities|FlowControl|Switch|SwitchonEnum_DialogueState _state_4
                    (:NewEnumerator0
                      (bind (_state_5 _optionindex) (CallFunction|AddDialogue "Джо" "Не знаю как попасть туда..." (Utilities|Array|MakeArray "Отдайте письмо мне, я доставлю куда надо" "Прости, не смогу помочь") 0 "/Game/Materials/testchar/Casual_Female_Anim_CharacterArmature_Defeat_Montage.Casual_Female_Anim_CharacterArmature_Defeat_Montage"))
                      (switch Utilities|FlowControl|Switch|SwitchonEnum_DialogueState _state_5
                        (:NewEnumerator0
                          (switch int _optionindex
                            (:0
                              (bind _state_6 (CallFunction|AddDialogue "Джо" "Правда?! Большое вам спасибо" 0 0 "/Game/Materials/testchar/Casual_Female_Anim_CharacterArmature_Victory_Montage.Casual_Female_Anim_CharacterArmature_Victory_Montage"))
                              (switch Utilities|FlowControl|Switch|SwitchonEnum_DialogueState _state_6
                                (:NewEnumerator0
                                  (bind _state_7 (CallFunction|AddDialogue "Джо" "Нужно доставить человеку по имени Лейла" 0 0 "/Game/Materials/testchar/Casual_Female_Anim_CharacterArmature_Victory_Montage.Casual_Female_Anim_CharacterArmature_Victory_Montage"))
                                  (switch Utilities|FlowControl|Switch|SwitchonEnum_DialogueState _state_7
                                    (:NewEnumerator0
                                      (CallFunction|CloseConversation)
                                      (CallFunction|SetDialogueBranch "Дал задание" "NewEnumerator0"))))))
                            (:1
                              (bind _state_8 (CallFunction|AddDialogue "Джо" "Что же делать...." 0 0 "/Game/Materials/testchar/Casual_Female_Anim_CharacterArmature_Defeat_Montage.Casual_Female_Anim_CharacterArmature_Defeat_Montage"))
                              (switch Utilities|FlowControl|Switch|SwitchonEnum_DialogueState _state_8
                                (:NewEnumerator0
                                  (CallFunction|RemoveDialogueProgress 1)
                                  (CallFunction|CloseConversation))))))))))))))
        (:NewEnumerator1
          (AI|Navigation|SimpleMovetoActor (AI|GetAIController (Components|GetOwner)) (Game|Player|GetPlayerPawn 0)))))
    (:Дал%20задание
      (bind _returnvalue (Actor|GetActorOfClass "/Game/Dialogue/BP_NPCTest.BP_NPCTest_C"))
      (if (Variables|/Game/Dialogue/AC_DialogueTest.AC_DialogueTest_C|GetLetterDeliv (Variables|/Game/Dialogue/BP_NPCTest.BP_NPCTest_C|GetAC_DialogueTest _returnvalue))
        (bind _state_9 (CallFunction|AddDialogue "Алекс" "Я доставил письмо" :!label _label))
        (switch Utilities|FlowControl|Switch|SwitchonEnum_DialogueState _state_9
          (:NewEnumerator0
            (bind _state_10 (CallFunction|AddDialogue "Алекс" "Спасибо большое!"))
            (switch Utilities|FlowControl|Switch|SwitchonEnum_DialogueState _state_10
              (:NewEnumerator0
                (CallFunction|CloseConversation)
                (CallFunction|SetDialogueBranch "Доставил" "NewEnumerator0")))))
        (else
          (bind (_state_11 _optionindex_2) (CallFunction|AddDialogue "Джо" "Ты уже доставил письмо?" (Utilities|Array|MakeArray "Нет, я пока не доставил" "А ты случаем не знаешь кого то кто хорошо знает этот остров?")))
          (switch Utilities|FlowControl|Switch|SwitchonEnum_DialogueState _state_11
            (:NewEnumerator0
              (switch int _optionindex_2
                (:0
                  (CallFunction|ClearDialogueProgress)
                  (CallFunction|CloseConversation))
                (:1
                  (bind _state_12 (CallFunction|AddDialogue "Джо" "Знаток этого острова - Сергей. Он знает это место вдоль и поперек"))
                  (switch Utilities|FlowControl|Switch|SwitchonEnum_DialogueState _state_12
                    (:NewEnumerator0
                      (bind _state_13 (CallFunction|AddDialogue "Джо" "Но однажды я сломал его параплан"))
                      (switch Utilities|FlowControl|Switch|SwitchonEnum_DialogueState _state_13
                        (:NewEnumerator0
                          (bind _state_14 (CallFunction|AddDialogue "Джо" "После этого он не подпускает меня к себе"))
                          (switch Utilities|FlowControl|Switch|SwitchonEnum_DialogueState _state_14
                            (:NewEnumerator0
                              (bind _state_15 (CallFunction|AddDialogue "Джо" "Может ты найдешь с ним общий язык"))
                              (switch Utilities|FlowControl|Switch|SwitchonEnum_DialogueState _state_15
                                (:NewEnumerator0
                                  (bind _state_16 (CallFunction|AddDialogue "Джо" "Он на верху этой скалы"))
                                  (switch Utilities|FlowControl|Switch|SwitchonEnum_DialogueState _state_16
                                    (:NewEnumerator0
                                      (CallFunction|CloseConversation)
                                      (CallFunction|SetDialogueBranch "После подсказки" "NewEnumerator0"))))))))))))))))))
    (:После%20подсказки
      (bind _returnvalue_2 (Actor|GetActorOfClass "/Game/Dialogue/BP_NPCTest.BP_NPCTest_C"))
      (if (Variables|/Game/Dialogue/AC_DialogueTest.AC_DialogueTest_C|GetLetterDeliv (Variables|/Game/Dialogue/BP_NPCTest.BP_NPCTest_C|GetAC_DialogueTest _returnvalue_2))
        (goto _label)
        (else
          (bind _state_17 (CallFunction|AddDialogue "Джо" (Utilities|Select :Index (Math|Random|RandomIntegerinRange 0 1) :Option%200 "Удачи в приключении!" :Option%201 "Будь осторожен!")))
          (switch Utilities|FlowControl|Switch|SwitchonEnum_DialogueState _state_17
            (:NewEnumerator0
              (CallFunction|ClearDialogueProgress)
              (CallFunction|CloseConversation))))))
    (:Доставил
      (bind _state_18 (CallFunction|AddDialogue "Джо" (Utilities|Select :Index (Math|Random|RandomIntegerinRange 0 1) :Option%200 "Удачи в приключении!" :Option%201 "Спасибо за помощь!")))
      (switch Utilities|FlowControl|Switch|SwitchonEnum_DialogueState _state_18
        (:NewEnumerator0
          (CallFunction|ClearDialogueProgress)
          (CallFunction|CloseConversation))))))