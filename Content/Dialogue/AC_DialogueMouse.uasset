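; Dialogue component for the Mouse NPC, scripting a branching conversation about Sara and the mouse's sunlight condition.
; Overrides Dialogue and switches on the active branch, chaining AddDialogue calls by state and chosen option.
; Endings close the conversation and either clear or roll back progress, or switch to "Being Stupid", which opens with a random brush-off.
; The joke line's Updated state also sends the mouse's AI controller toward the player.
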(fn Dialogue
  (|CallParentFunction)
  (switch name (Variables|Default|GetActiveDialogueBranch)
    (:Default
      (bind (_state _optionindex) (CallFunction|AddDialogue "Mouse" "Hello, traveller!" (Utilities|Array|MakeArray "Hello, do you know Sara?" "Hi, are you alright? You seem to be sick.")))
      (switch Utilities|FlowControl|Switch|SwitchonEnum_DialogueState _state
        (:NewEnumerator0
          (switch int _optionindex
            (:0
              (bind (_state_2 _optionindex_2) (CallFunction|AddDialogue "Mouse" "Yes! I know her! ... She is in the graveyard buried 6 ft in the ground" (Utilities|Array|MakeArray "What?" "You will be the one rotting, if you don't elobarate right now!")))
              (switch Utilities|FlowControl|Switch|SwitchonEnum_DialogueState _state_2
                (:NewEnumerator0
                  (switch int _optionindex_2
                    (:0
                      (bind _state_3 (CallFunction|AddDialogue "Mouse" "Whatever"))
                      (switch Utilities|FlowControl|Switch|SwitchonEnum_DialogueState _state_3
                        (:NewEnumerator0
                          (CallFunction|CloseConversation)
                          (CallFunction|SetDialogueBranch "Being stupid" "NewEnumerator0"))))
                    (:1
                      (bind _state_4 (CallFunction|AddDialogue "Mouse" "I am just joking, don't be so serious" (Utilities|Array|MakeArray "You better not do that again")))
                      (switch Utilities|FlowControl|Switch|SwitchonEnum_DialogueState _state_4
                        (:NewEnumerator0
                          (CallFunction|RemoveDialogueProgress 1)
                          (CallFunction|CloseConversation))
                        (:NewEnumerator1
                          (AI|Navigation|MovetoActor (AI|GetAIController (Components|GetOwner)) (Game|GetPlayerCharacter 0) -1.0 true true true 0))))))))
            (:1
              (bind _state_5 (CallFunction|AddDialogue "Mouse" "Ah. This. Sunlight gives burns, because of my condition. I can't find my potion for that." (Utilities|Array|MakeArray "Maybe i can find it for you")))
              (switch Utilities|FlowControl|Switch|SwitchonEnum_DialogueState _state_5
                (:NewEnumerator0
                  (CallFunction|ClearDialogueProgress)
                  (CallFunction|CloseConversation))))))))
    (:Being%20stupid
      (bind _state_6 (CallFunction|AddDialogue "Mouse" (Utilities|Select :Index (Math|Random|RandomIntegerinRange 0 1) :Option%200 "Get out" :Option%201 "Go away")))
      (switch Utilities|FlowControl|Switch|SwitchonEnum_DialogueState _state_6
        (:NewEnumerator0
          (CallFunction|AddDialogue "Player" "I just wanted to talk")
          (switch Utilities|FlowControl|Switch|SwitchonEnum_DialogueState "NewEnumerator0"
            (:NewEnumerator0
              (CallFunction|ClearDialogueProgress)
              (CallFunction|CloseConversation))))))))