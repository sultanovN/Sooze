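; Dialogue component for NPC Sergey, who mistakes Alex for someone who pushed him off a cliff, then discusses borrowing his paraglider or crossing the island.
; Overrides Dialogue, calls the parent, then switches on ActiveDialogueBranch, chaining AddDialogue lines with player options and occasional montages.
; Both opening replies converge, and both final choices close the conversation and set the paraglider-received branch.
; That branch plays one of two random remarks, then clears progress.
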(fn Dialogue
  (|CallParentFunction)
  (switch name (Variables|Default|GetActiveDialogueBranch)
    (:Default
      (bind (_state _optionindex) (CallFunction|AddDialogue "Сергей" "Уйди отсюда!" (Utilities|Array|MakeArray "Простите?" "Не кричи на меня") 0 "/Game/Materials/testchar/Casual_Female_Anim_CharacterArmature_SwordSlash_Montage.Casual_Female_Anim_CharacterArmature_SwordSlash_Montage"))
      (switch Utilities|FlowControl|Switch|SwitchonEnum_DialogueState _state
        (:NewEnumerator0
          (switch int _optionindex
            (:0
              (bind _state_2 (CallFunction|AddDialogue "Сергей" "Ой, извини я тебя перепутал с кем то другим"))
              (switch Utilities|FlowControl|Switch|SwitchonEnum_DialogueState _state_2
                (:NewEnumerator0
                  _)))
            (:1
              (bind _state_3 (CallFunction|AddDialogue "Сергей" "Прости, пожалуйста! Я перепутал тебя с другим!" 0 0 "/Game/Materials/testchar/Casual_Female_Anim_CharacterArmature_PickUp_Montage.Casual_Female_Anim_CharacterArmature_PickUp_Montage"))
              (switch Utilities|FlowControl|Switch|SwitchonEnum_DialogueState _state_3
                (:NewEnumerator0
                  _))))
          (bind _state_4 (CallFunction|AddDialogue "Алекс" "Вы подумали что я тот человек который сломал параплан?"))
          (switch Utilities|FlowControl|Switch|SwitchonEnum_DialogueState _state_4
            (:NewEnumerator0
              (bind _state_5 (CallFunction|AddDialogue "Сергей" "Параплан?..."))
              (switch Utilities|FlowControl|Switch|SwitchonEnum_DialogueState _state_5
                (:NewEnumerator0
                  (bind _state_6 (CallFunction|AddDialogue "Сергей" "Параплан это сущая мелочь, он меня с обрыва столкнул!!!"))
                  (switch Utilities|FlowControl|Switch|SwitchonEnum_DialogueState _state_6
                    (:NewEnumerator0
                      (bind _state_7 (CallFunction|AddDialogue "Алекс" "Я боялся с парапланом прыгнуть "))
                      (switch Utilities|FlowControl|Switch|SwitchonEnum_DialogueState _state_7
                        (:NewEnumerator0
                          (bind _state_8 (CallFunction|AddDialogue "Алекс" "А он захотел подбодрить меня знаешь ли"))
                          (switch Utilities|FlowControl|Switch|SwitchonEnum_DialogueState _state_8
                            (:NewEnumerator0
                              (bind _state_9 (CallFunction|AddDialogue "Алекс" "Ох..."))
                              (switch Utilities|FlowControl|Switch|SwitchonEnum_DialogueState _state_9
                                (:NewEnumerator0
                                  (bind _state_10 (CallFunction|AddDialogue "Сергей" "Он конечно это случайно сделал"))
                                  (switch Utilities|FlowControl|Switch|SwitchonEnum_DialogueState _state_10
                                    (:NewEnumerator0
                                      (bind (_state_11 _optionindex_2) (CallFunction|AddDialogue "Сергей" "Так ты что то хотел от меня?" (Utilities|Array|MakeArray "Можно у тебя одолжить параплан?" "Хотел узнать как можно перейти на другу сторону острова")))
                                      (switch Utilities|FlowControl|Switch|SwitchonEnum_DialogueState _state_11
                                        (:NewEnumerator0
                                          (switch int _optionindex_2
                                            (:0
                                              (bind _state_12 (CallFunction|AddDialogue "Сергей" "Да, конечно"))
                                              (switch Utilities|FlowControl|Switch|SwitchonEnum_DialogueState _state_12
                                                (:NewEnumerator0
                                                  (bind _state_13 (CallFunction|AddDialogue "Сергей" "Все равно в ближайшее время не смогу ей воспользоваться"))
                                                  (switch Utilities|FlowControl|Switch|SwitchonEnum_DialogueState _state_13
                                                    (:NewEnumerator0
                                                      (CallFunction|CloseConversation)
                                                      (CallFunction|SetDialogueBranch "Получил параплан" "NewEnumerator0"))))))
                                            (:1
                                              (bind _state_14 (CallFunction|AddDialogue "Сергей" "Есть мост ведущий на ту сторону"))
                                              (switch Utilities|FlowControl|Switch|SwitchonEnum_DialogueState _state_14
                                                (:NewEnumerator0
                                                  (bind _state_15 (CallFunction|AddDialogue "Сергей" "Ну или парапланом можешь перелететь"))
                                                  (switch Utilities|FlowControl|Switch|SwitchonEnum_DialogueState _state_15
                                                    (:NewEnumerator0
                                                      (CallFunction|CloseConversation)
                                                      (CallFunction|SetDialogueBranch "Получил параплан" "NewEnumerator0"))))))))))))))))))))))))))
    (:Получил%20параплан
      (bind _state_16 (CallFunction|AddDialogue "Сергей" (Utilities|Select :Index (Math|Random|RandomIntegerinRange 0 1) :Option%200 "Ну как? Оседлал ветер?" :Option%201 "После параплана ходьба невыносимо медленная")))
      (switch Utilities|FlowControl|Switch|SwitchonEnum_DialogueState _state_16
        (:NewEnumerator0
          (CallFunction|ClearDialogueProgress)
          (CallFunction|CloseConversation))))))