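; Dialogue component for the NPC Fred, who offers to teach climbing and guides the player through a short tutorial in Russian.
; It overrides Dialogue and switches on the active branch, chaining AddDialogue lines with Alex's replies, montages and a win sound.
; Each stage sets the next branch, from small platform through large platform to completion, ending in random farewells.
; Disconnected English "Mouse" dialogue nodes remain unused.
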(fn Dialogue
  (|CallParentFunction)
  (switch name (Variables|Default|GetActiveDialogueBranch)
    (:Default
      (bind _state (CallFunction|AddDialogue "Фред" "Привет, путешественник!"))
      (switch Utilities|FlowControl|Switch|SwitchonEnum_DialogueState _state
        (:NewEnumerator0
          (bind _state_2 (CallFunction|AddDialogue "Фред" " Не хочешь научится чему то новому?"))
          (switch Utilities|FlowControl|Switch|SwitchonEnum_DialogueState _state_2
            (:NewEnumerator0
              (bind _state_3 (CallFunction|AddDialogue "Алекс" "А чему ты можешь научить?"))
              (switch Utilities|FlowControl|Switch|SwitchonEnum_DialogueState _state_3
                (:NewEnumerator0
                  (bind _state_4 (CallFunction|AddDialogue "Фред" "Тому ради чего приходят любители горячих ощущений!"))
                  (switch Utilities|FlowControl|Switch|SwitchonEnum_DialogueState _state_4
                    (:NewEnumerator0
                      (bind _state_5 (CallFunction|AddDialogue "Фред" "Скалолазанию!" 0 0 "/Game/Materials/testchar/Casual_Female_Anim_CharacterArmature_Victory_Montage.Casual_Female_Anim_CharacterArmature_Victory_Montage"))
                      (switch Utilities|FlowControl|Switch|SwitchonEnum_DialogueState _state_5
                        (:NewEnumerator0
                          (bind _state_6 (CallFunction|AddDialogue "Фред" "Попробуй поднятся на эту малую платформу."))
                          (switch Utilities|FlowControl|Switch|SwitchonEnum_DialogueState _state_6
                            (:NewEnumerator0
                              (CallFunction|CloseConversation)
                              (CallFunction|SetDialogueBranch "Малая платформа" "NewEnumerator0"))))))))))))))
    (:Малая%20платформа
      (bind _state_7 (CallFunction|AddDialogue "Фред" "Молодец! Быстро учишься"))
      (switch Utilities|FlowControl|Switch|SwitchonEnum_DialogueState _state_7
        (:NewEnumerator0
          (bind _state_8 (CallFunction|AddDialogue "Фред" "Теперь попробуй взабраться на большую"))
          (switch Utilities|FlowControl|Switch|SwitchonEnum_DialogueState _state_8
            (:NewEnumerator0
              (CallFunction|CloseConversation)
              (CallFunction|SetDialogueBranch "Большая платформа" "NewEnumerator0"))))))
    (:Большая%20платформа
      (bind _state_9 (CallFunction|AddDialogue "Фред" "Отлично! У тебя большой потенциал" 0 "/Game/Sound/Win.Win" "/Game/Materials/testchar/Casual_Female_Anim_CharacterArmature_Victory_Montage.Casual_Female_Anim_CharacterArmature_Victory_Montage"))
      (switch Utilities|FlowControl|Switch|SwitchonEnum_DialogueState _state_9
        (:NewEnumerator0
          (bind _state_10 (CallFunction|AddDialogue "Фред" "Ты прошел обучение, теперь можешь идти покорять горы!"))
          (switch Utilities|FlowControl|Switch|SwitchonEnum_DialogueState _state_10
            (:NewEnumerator0
              (CallFunction|CloseConversation)
              (CallFunction|SetDialogueBranch "Прошел обучение" "NewEnumerator0"))))))
    (:Прошел%20обучение
      (bind _state_11 (CallFunction|AddDialogue "Фред" "Как дела? Покорил остров?"))
      (switch Utilities|FlowControl|Switch|SwitchonEnum_DialogueState _state_11
        (:NewEnumerator0
          (bind _state_12 (CallFunction|AddDialogue "Алекс" "Хорошо, я пока только начал изучать остров"))
          (switch Utilities|FlowControl|Switch|SwitchonEnum_DialogueState _state_12
            (:NewEnumerator0
              (CallFunction|CloseConversation)
              (CallFunction|SetDialogueBranch "Удачи" "NewEnumerator0"))))))
    (:Удачи
      (bind _state_13 (CallFunction|AddDialogue "Фред" (Utilities|Select :Index (Math|Random|RandomIntegerinRange 0 1) :Option%200 "Удачи в приключении!" :Option%201 "Будь осторожен!")))
      (switch Utilities|FlowControl|Switch|SwitchonEnum_DialogueState _state_13
        (:NewEnumerator0
          (CallFunction|ClearDialogueProgress)
          (CallFunction|CloseConversation))))))