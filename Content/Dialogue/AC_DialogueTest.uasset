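; Test dialogue component scripting a short Russian-language exchange in which Алекс delivers a letter to Лейла.
; The Dialogue override switches on the active branch and chains AddDialogue nodes through their Pass Through state.
; Finishing the default branch sets LetterDeliv, closes the conversation and switches to "Given bleach", where Лейла only gives thanks for the delivery.
; An Updated state on Лейла's first line sets the owner's skeletal mesh to Animation Blueprint mode.
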(event EventBeginPlay
  (|CallParentFunction) ; This node is disabled and will not be called.\nDrag off pins to build functionality.
)

(event EventTick
  (params (DeltaSeconds :type Float%20%28single-precision%29)))

(fn Dialogue
  (|CallParentFunction)
  (switch name (Variables|Default|GetActiveDialogueBranch)
    (:Default
      (bind _state (CallFunction|AddDialogue "Алекс" "Привет тебе хотели передать письмо"))
      (switch Utilities|FlowControl|Switch|SwitchonEnum_DialogueState _state
        (:NewEnumerator0
          (bind _state_2 (CallFunction|AddDialogue "Лейла" "Письмо?"))
          (switch Utilities|FlowControl|Switch|SwitchonEnum_DialogueState _state_2
            (:NewEnumerator0
              (bind _state_3 (CallFunction|AddDialogue "Лейла" "Спасибо, я прочитаю"))
              (switch Utilities|FlowControl|Switch|SwitchonEnum_DialogueState _state_3
                (:NewEnumerator0
                  (Variables|Default|SetLetterDeliv true)
                  (CallFunction|CloseConversation)
                  (CallFunction|SetDialogueBranch "Given bleach" "NewEnumerator0"))))
            (:NewEnumerator1
              (Components|Animation|SetAnimationMode (Actor|GetComponentbyClass (Components|GetOwner) "/Script/Engine.SkeletalMeshComponent") "AnimationBlueprint" false))))))
    (:Given%20bleach
      (bind _state_4 (CallFunction|AddDialogue "Лейла" "Спасибо за доставку"))
      (switch Utilities|FlowControl|Switch|SwitchonEnum_DialogueState _state_4
        (:NewEnumerator0
          (CallFunction|CloseConversation))))))