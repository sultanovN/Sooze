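; BP_NPCBase is a base Blueprint for dialogue NPCs that shows a character name label and reports when a conversation ends.
; The construction script writes CharacterName into the TxtCharacterName text component.
; SetInteractableState shows or hides that label according to whether interaction is available.
; ConversationClosed passes the event back to the stored InteractInstigator through ConversationClosedMessage.
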(event EventConversationClosed
  (Class|BPIInteractable|ConversationClosed(Message) (Variables|Default|GetInteractInstigator)))

(event EventSetInteractableState
  (params (bCanShowInteract :type Boolean))
  (bind _txt_charactername (Variables|Default|GetTxt_CharacterName))
  (if bCanShowInteract
    (Rendering|SetVisibility _txt_charactername true false)
    (else
      (Rendering|SetVisibility _txt_charactername false false))))

(fn ConstructionScript
  (Rendering|Components|TextRender|SetText (Variables|Default|GetTxt_CharacterName) (Variables|Default|GetCharacterName)))