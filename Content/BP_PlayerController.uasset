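; Player controller Blueprint that handles the pause menu and switches input between UI and gameplay.
; The pause input lazily creates and caches a UINav pause menu widget, then either shows it and pauses the game or returns it to its parent and unpauses.
; Root widget added and removed events toggle the mouse cursor and switch between UI-only and game-only input modes.
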(event Input|EnhancedActionEvents|EnhancedInputActionIA_Pause
  (params (ActionValue :type Boolean) (ElapsedSeconds :type Float%20%28double-precision%29) (TriggeredSeconds :type Float%20%28double-precision%29) (InputAction :type Input%20Action%20Object%20Reference :default "/Game/ThirdPerson/Input/Actions/IA_Pause.IA_Pause"))
  ;[0.01938 0.01938 0.01938] PauseGame
  (:Started
    (Utilities|IsValid (Variables|Default|GetPauseRef)
      (:Is%20Valid
        _)
      (:Is%20Not%20Valid
        (bind _returnvalue (UserInterface|CreateWidget "/Game/UI/Menu/WB_UINavPauseMenu.WB_UINavPauseMenu_C" self))
        (Variables|Default|SetPauseRef _returnvalue)))
    (if (Game|IsGamePaused)
      (Class|UINavWidget|ReturntoParent (Variables|Default|GetPauseRef) false)
      (Game|SetGamePaused false)
      (else
        (UserInterface|Viewport|AddtoViewport (Variables|Default|GetPauseRef) 0)
        (Game|SetGamePaused true)))))

(event EventOnRootWidgetAdded
  (Variables|Default|SetbShowMouseCursor true)
  (Input|SetInputModeUIOnly self 0 "DoNotLock" false))

(event EventOnRootWidgetRemoved
  (Variables|Default|SetbShowMouseCursor false)
  (Input|SetInputModeGameOnly self false))

(fn ConstructionScript)